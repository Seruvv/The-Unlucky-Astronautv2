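; BP_GA_Tile_Box_02 is an Advanced Turn Based Tile Toolkit tile that sends the game into an encounter.
; On BeginPlay it binds to the grid manager's unit end-movement simulate event and compares grid indices when that fires.
; On a match it copies its encounter, attack, interact and flee descriptions plus air supply status into BP_Instance_ATBTT, then opens EncounterMap.
; The game instance carries that data across the level change.
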(event Custom|Go%20To%20Encounter
  (params (Unit :type BP%20Unit%20Object%20Reference) (GridIndex :type Integer))
  (if (== GridIndex (Variables|Default|GetGridIndex))
    (bind _asbp_instance_atbtt (Utilities|Casting|CastToBP_Instance_ATBTT (Game|GetGameInstance)))
    (Development|PrintString "Cool")
    (Utilities|FlowControl|Sequence
      (:then_0
        (Variables|/Game/AdvancedTurnBasedTileToolkit/Maps/MP/Core/BP_Instance_ATBTT.BP_Instance_ATBTT_C|SetencounterDes _asbp_instance_atbtt (Variables|Default|GetencounterDes)))
      (:then_1
        (Variables|/Game/AdvancedTurnBasedTileToolkit/Maps/MP/Core/BP_Instance_ATBTT.BP_Instance_ATBTT_C|SetattackDes _asbp_instance_atbtt (Variables|Default|GetattackDes)))
      (:then_2
        (Variables|/Game/AdvancedTurnBasedTileToolkit/Maps/MP/Core/BP_Instance_ATBTT.BP_Instance_ATBTT_C|SetinteractDes _asbp_instance_atbtt (Variables|Default|GetinteractDes)))
      (:then_3
        (Variables|/Game/AdvancedTurnBasedTileToolkit/Maps/MP/Core/BP_Instance_ATBTT.BP_Instance_ATBTT_C|SetfleeDes _asbp_instance_atbtt (Variables|Default|GetfleeDes)))
      (:then_4
        (Variables|/Game/AdvancedTurnBasedTileToolkit/Maps/MP/Core/BP_Instance_ATBTT.BP_Instance_ATBTT_C|SetairSupplyStatus _asbp_instance_atbtt (Variables|Default|GetairSupply)))
      (:then_5
        (Game|OpenLevel(byName) "EncounterMap")))))

(event EventBeginPlay
  (EventDispatchers|BindEventtoOnUnitEndMovementSimulate (Variables|Default|GetGridManagerRef) (delegate Custom|Go%20To%20Encounter)))

(fn ConstructionScript
  (|CallParentFunction))