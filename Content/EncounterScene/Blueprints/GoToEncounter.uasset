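; Grid-placed encounter trigger that sends the game to the EncounterMap level when a unit's movement ends on its grid index.
; It listens to the grid manager's end-of-movement event, then saves the unit's player values and its own Idle, Attack, Interact and Flee encounter states to the game instance.
; The level change runs as a queued action, with AnimateAction opening the map and signalling the game state that the action ended.
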(event Custom|Go%20To%20Encounter
  (params (Unit :type BP%20Unit%20Object%20Reference) (GridIndex :type Integer))
  (if (== (Variables|Default|GetGridIndex) GridIndex)
    (CallFunction|SetEncounterValues Unit GridIndex)
    (Utilities|QueueAction false self "GoToEncounter" false -1 false 0.0)))

(event EventBeginPlay
  (CallFunction|CheckPlayerStartGridIndex)
  (EventDispatchers|BindEventtoOnUnitEndMovementSimulate (Variables|Default|GetGridManagerRef) (delegate Custom|Go%20To%20Encounter)))

(event EventAnimateAction
  (params (Action :type F%20Action%20Structure))
  (Game|OpenLevel(byName) "EncounterMap")
  (Class|BPIAction|EndAction(Message) (Game|GetGameState)))

(fn ConstructionScript
  (|CallParentFunction))

(fn CheckPlayerStartGridIndex
  (bind _asbp_instance_atbtt (Utilities|Casting|CastToBP_Instance_ATBTT (Game|GetGameInstance)))
  (return (== (.currentGridIndex (Utilities|Struct|BreakPlayerValuesStruct (Variables|/Game/AdvancedTurnBasedTileToolkit/Maps/MP/Core/BP_Instance_ATBTT.BP_Instance_ATBTT_C|GetPlayer _asbp_instance_atbtt))) (Variables|Default|GetGridIndex))))

(fn SetEncounterValues
  (params (Unit :type BP%20Unit%20Object%20Reference) (unitGridIndex :type Integer))
  (bind _asbp_instance_atbtt (Utilities|Casting|CastToBP_Instance_ATBTT (Game|GetGameInstance)))
  (Utilities|FlowControl|Sequence
    (:then_0
      (bind _playervalues (Default|SetPlayerValuesStruct (Variables|/Game/AdvancedTurnBasedTileToolkit/Core/Units/BP_Unit.BP_Unit_C|GetPlayerValues Unit) unitGridIndex))
      (Variables|/Game/AdvancedTurnBasedTileToolkit/Maps/MP/Core/BP_Instance_ATBTT.BP_Instance_ATBTT_C|Setplayer _asbp_instance_atbtt _playervalues))
    (:then_1
      (Variables|/Game/AdvancedTurnBasedTileToolkit/Maps/MP/Core/BP_Instance_ATBTT.BP_Instance_ATBTT_C|Setidle _asbp_instance_atbtt (Variables|Default|GetencounterIdleState)))
    (:then_2
      (Variables|/Game/AdvancedTurnBasedTileToolkit/Maps/MP/Core/BP_Instance_ATBTT.BP_Instance_ATBTT_C|Setattack _asbp_instance_atbtt (Variables|Default|GetencounterAttackState)))
    (:then_3
      (Variables|/Game/AdvancedTurnBasedTileToolkit/Maps/MP/Core/BP_Instance_ATBTT.BP_Instance_ATBTT_C|Setinteract _asbp_instance_atbtt (Variables|Default|GetencounterInteractState)))
    (:then_4
      (Variables|/Game/AdvancedTurnBasedTileToolkit/Maps/MP/Core/BP_Instance_ATBTT.BP_Instance_ATBTT_C|Setflee _asbp_instance_atbtt (Variables|Default|GetencounterFleeState)))))