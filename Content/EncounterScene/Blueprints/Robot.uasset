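; Robot Blueprint for the encounter scene, driven by a RobotStruct holding type, lives, storage capability and resources.
; CollectResources appends a resource while the resource array is below storage capability, otherwise printing a refusal.
; LoseLife prints a destruction message naming the robot type when one less than current lives equals zero, but never stores the decrement or destroys the robot.
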(fn ConstructionScript)

(fn CollectResources
  (params (resource :type feedbacks_resources%20Enum :default "NewEnumerator6"))
  (bind _robotstruct (Variables|Default|GetrobotStruct))
  (bind (_robottype _maxlifes _currentlifes _storagecapability _speed _resources) (Utilities|Struct|BreakRobotStruct _robotstruct))
  (if (> _storagecapability (Utilities|Array|Length _resources))
    (Utilities|Array|Add _resources resource)
    (else
      (Development|PrintString "Can't Take it"))))

(fn LoseLife
  (bind _robotstruct (Variables|Default|GetrobotStruct))
  (bind (_robottype _maxlifes _currentlifes) (Utilities|Struct|BreakRobotStruct _robotstruct))
  (if (== (- _currentlifes 1) 0)
    (Development|PrintString (Utilities|String|Append (Utilities|String|EnumtoString _robottype) " is Destroyed"))))