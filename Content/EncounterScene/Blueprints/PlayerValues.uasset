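; PlayerValues holds the player's encounter-scene state: robots, robot in use, map state, air supply and held ship racks.
; SetPlayerValuesStruct packs that state and a supplied grid index into a struct, and GetPlayerValuesFromStruct restores the variables from one and returns them.
; Helpers replace the map state, mark a map piece as revealed at a grid index, and check the robot list for a requested type.
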(fn SetCurrentMapState
  (params (Map :type Array%20of%20Map%20Piece%20Structures))
  (Variables|Default|SetmapState Map))

(fn ChangeMap
  (params (Map :type Array%20of%20Map%20Piece%20Structures) (gridIndex :type Integer))
  (Utilities|Array|SetArrayElem Map gridIndex (Utilities|Struct|MakeMapPiece (.mapIndex (Utilities|Struct|BreakMapPiece (Utilities|Array|Get(acopy) Map gridIndex))) true)))

(fn ChooseRobot
  (params (robots :type Array%20of%20Robot%20Struct%20Structures) (robotType :type Robot%20Struct%20Structure))
  (if (not (== (Utilities|Array|Length robots) 0))
    (for _array_element robots
      (if (== (.robotType (Utilities|Struct|BreakRobotStruct _array_element)) (.robotType (Utilities|Struct|BreakRobotStruct robotType)))
        (return robotType)))))

(fn SetPlayerValuesStruct
  (params (gridIndex :type Integer))
  (bind _structout (Utilities|Struct|SetmembersinPlayerValuesStruct (Utilities|Struct|MakePlayerValuesStruct (Variables|Default|Getrobots) (Variables|Default|GetrobotInUse) (Variables|Default|GetmapState) (Variables|Default|GetmaxAirSupply) (Variables|Default|GetcurrentAirSupply) gridIndex (Variables|Default|GetholdingShipracks))))
  (return _structout))

(fn GetPlayerValuesfromStruct
  (params (playerValues :type Player%20Values%20Struct%20Structure))
  (bind (_robotslist _robotinuse _mapstate _maxairsupply _currentairsupply _currentgridindex _shipracks) (Utilities|Struct|BreakPlayerValuesStruct playerValues))
  (Utilities|FlowControl|Sequence
    (:then_0
      (bind _output_get (Variables|Default|Setrobots _robotslist)))
    (:then_1
      (bind _output_get_2 (Variables|Default|SetrobotInUse _robotinuse)))
    (:then_2
      (bind _output_get_3 (Variables|Default|SetmapState _mapstate)))
    (:then_3
      (bind _output_get_4 (Variables|Default|SetmaxAirSupply _maxairsupply)))
    (:then_4
      (bind _output_get_5 (Variables|Default|SetcurrentAirSupply _currentairsupply)))
    (:then_5
      (bind _output_get_6 (Variables|Default|SetholdingShipracks _shipracks)))
    (:then_6
      (return _output_get _output_get_2 _output_get_3 _output_get_4 _output_get_5 _output_get_6 _currentgridindex))))