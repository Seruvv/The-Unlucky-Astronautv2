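; Test-settings actor for the encounter scene that seeds the game instance with debug data on BeginPlay.
; When its Testing flag is set, it writes Idle, Attack, Interact and Flee values into BP_Instance_ATBTT.
; It also builds a Player values struct from a single test robot, one map piece and preset air supply.
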(event EventBeginPlay
  (bind _robot (Variables|Default|GetRobot))
  (bind _asbp_instance_atbtt (Utilities|Casting|CastToBP_Instance_ATBTT (Game|GetGameInstance)))
  (if (Variables|Default|Gettesting)
    (Utilities|FlowControl|Sequence
      (:then_0
        (Variables|/Game/AdvancedTurnBasedTileToolkit/Maps/MP/Core/BP_Instance_ATBTT.BP_Instance_ATBTT_C|Setidle _asbp_instance_atbtt (Variables|Default|Getidle)))
      (:then_1
        (Variables|/Game/AdvancedTurnBasedTileToolkit/Maps/MP/Core/BP_Instance_ATBTT.BP_Instance_ATBTT_C|Setattack _asbp_instance_atbtt (Variables|Default|Getattack)))
      (:then_2
        (Variables|/Game/AdvancedTurnBasedTileToolkit/Maps/MP/Core/BP_Instance_ATBTT.BP_Instance_ATBTT_C|Setinteract _asbp_instance_atbtt (Variables|Default|Getinteract)))
      (:then_3
        (Variables|/Game/AdvancedTurnBasedTileToolkit/Maps/MP/Core/BP_Instance_ATBTT.BP_Instance_ATBTT_C|Setflee _asbp_instance_atbtt (Variables|Default|Getflee)))
      (:then_4
        (Variables|/Game/AdvancedTurnBasedTileToolkit/Maps/MP/Core/BP_Instance_ATBTT.BP_Instance_ATBTT_C|SetPlayer _asbp_instance_atbtt (Utilities|Struct|MakePlayerValuesStruct (Utilities|Array|MakeArray _robot) _robot (Utilities|Array|MakeArray (Variables|Default|GetmapPiece)) 10 5))))))

(fn ConstructionScript)